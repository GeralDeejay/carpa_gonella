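; BP_DMXPointLight is a DMX fixture actor that drives a Point Light from received DMX fixture patch data.
; On patch reception it reads normalized attribute values and looks them up to set the light's RGB color and its intensity as a fraction of MaxIntensity.
; The construction script sets the light to MaxIntensity as its initial brightness.
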(event `self.DMX.OnFixturePatchReceived`
  (params (FixturePatch :type "DMXEntityFixturePatch Object Reference") (ValuePerAttribute :type "DMXNormalizedAttributeValueMap Structure (by ref)"))
  ;[0.5925 0.6093 1] Map DMX values between 0 and 1
  (bind _normalizedattributesvalues (`DMXEntityFixturePatch.GetNormalizedAttributesValues` FixturePatch))
  ;[0.5925 0.6093 1] Change color and intensity of Point Light
  (`LightComponent.SetLightColor` (`self.PointLight`) (make `LinearColor` (`BlueprintMapLibrary.Map_Find` (break `DMXNormalizedAttributeValueMap` _normalizedattributesvalues) (struct :`Name` "Red")) (`BlueprintMapLibrary.Map_Find` (break `DMXNormalizedAttributeValueMap` _normalizedattributesvalues) (struct :`Name` "Green")) (`BlueprintMapLibrary.Map_Find` (break `DMXNormalizedAttributeValueMap` _normalizedattributesvalues) (struct :`Name` "Blue")) 1.0) true)
  (`LightComponent.SetIntensity` (`self.PointLight`) (* (`BlueprintMapLibrary.Map_Find` (break `DMXNormalizedAttributeValueMap` _normalizedattributesvalues) (struct :`Name` "Dimmer")) (`self.MaxIntensity`))))

(fn `UserConstructionScript`
  (`LightComponent.SetIntensity` (`self.PointLight`) (`self.MaxIntensity`)))