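; Scene capture actor that produces a downsampled, blurred copy of its captured view in a destination render target.
; The construction script creates a blur material instance and a chain of clamped render targets at successively halved resolutions, capturing into the first and appending DestRT last.
; DestRT is resized to the smallest step during construction and again at BeginPlay.
; Each Tick draws every target into the next through the blur material, forming a progressive downsample blur.
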(event `self.ReceiveBeginPlay`
  (`self.ApplySizeToDestRT`))

(event `self.ReceiveTick`
  (params (DeltaSeconds :type "Float (single-precision)"))
  (bind _blurmaterialinstance (`self.BlurMaterialInstance`))
  ;[1 1 1] Downsample Render Passes
  (for _index (range (+ (- (`KismetArrayLibrary.Array_Length` (`self.DownSamplesRT`)) 2) 1))
    (`MaterialInstanceDynamic.SetTextureParameterValue` _blurmaterialinstance "Texture" (`|GetArrayItem` (`self.DownSamplesRT`) _index))
    (`MaterialInstanceDynamic.SetScalarParameterValue` _blurmaterialinstance "Blur Strength" (`self.Blur Strength`))
    (`KismetRenderingLibrary.DrawMaterialToRenderTarget` (`|GetArrayItem` (`self.DownSamplesRT`) (+ _index 1)) _blurmaterialinstance)))

(fn `ApplySizeToDestRT`
  (bind _returnvalue (`KismetMathLibrary.MultiplyMultiply_FloatFloat` 2.0 (`KismetMathLibrary.Conv_IntToDouble` (`self.DownSamplesCount`))))
  (`KismetRenderingLibrary.ResizeRenderTarget2D` (`self.DestRT`) (`KismetMathLibrary.FTrunc` (/ (`self.SceneCaptureWidth`) _returnvalue)) (`KismetMathLibrary.FTrunc` (/ (`self.SceneCaptureHeight`) _returnvalue))))

(fn `UserConstructionScript`
  (locals (Counter :type Integer :default 1))
  ;[1 1 1] Create Blur Material Dynamic Instance
  (bind _returnvalue (`KismetMaterialLibrary.CreateDynamicMaterialInstance` (`self.BlurMaterial`)))
  (set `self.BlurMaterialInstance` _returnvalue)
  ;[1 1 1] Create a series of Downsample Rendertargets
  (for _index (range (`self.DownSamplesCount`))
    (bind _returnvalue_2 (`KismetMathLibrary.MultiplyMultiply_FloatFloat` 2.0 (`KismetMathLibrary.Conv_IntToDouble` _index)))
    (bind _returnvalue_3 (`KismetRenderingLibrary.CreateRenderTarget2D` (/ (`self.SceneCaptureWidth`) _returnvalue_2) (/ (`self.SceneCaptureHeight`) _returnvalue_2)))
    ;[1 1 1] Set Wrap to Clamp
    (set `TextureRenderTarget2D.AddressX` "TA_Clamp" _returnvalue_3)
    (set `TextureRenderTarget2D.AddressY` "TA_Clamp" _returnvalue_3)
    (`KismetArrayLibrary.Array_Add` (`self.DownSamplesRT`) _returnvalue_3))
  ;[1 1 1] Set Scene Capture Rendertarget to first in array
  (set `SceneCaptureComponent2D.TextureTarget` (`|GetArrayItem` (`self.DownSamplesRT`)) (`self.SceneCaptureComponent2D`))
  ;[1 1 1] Set resolution of Destination Rendertarget
  (`self.ApplySizeToDestRT`)
  (`KismetArrayLibrary.Array_Add` (`self.DownSamplesRT`) (`self.DestRT`)))